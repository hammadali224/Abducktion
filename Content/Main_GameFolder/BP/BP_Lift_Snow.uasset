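; BP_Lift_Snow is a moving lift that shuttles its Box component back and forth between its relative origin and MovementLocation.
; On BeginPlay, the Intp timeline starts with its play rate set from Duration and lerps the Box's relative location.
; When the timeline finishes it flips direction, looping the motion.
; An overlap on the Bottom component during the return trip sends the lift forward again early.
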(event `self.Bottom.OnComponentBeginOverlap`
  (params (OverlappedComponent :type "PrimitiveComponent Object Reference") (OtherActor :type "Actor Object Reference") (OtherComp :type "PrimitiveComponent Object Reference") (OtherBodyIndex :type Integer) (bFromSweep :type Boolean) (SweepResult :type "HitResult Structure (by ref)"))
  ;[1 1 1] Reverse Direction when bottom hits
  (if (`TimelineComponent.IsReversing` (`self.Intp`))
    (`self.Forward`)))

(event `self.ReceiveBeginPlay`
  ;[1 1 1] Movement Mechanism & Initialize Sprite Type
  (`TimelineComponent.SetPlayRate` (`self.Intp`) (/ 1.0 (`self.Duration`)))
  (bind (_direction _linearintp) (`Timeline|Intp` :!via `PlayFromStart` :!label _label)
    (:`Update`
      (`SceneComponent.K2_SetRelativeLocation` (`self.Box`) (`KismetMathLibrary.VLerp` (0.0 0.0 0.0) (`self.MovementLocation`) _linearintp) false false))
    (:`Finished`
      (switch `ETimelineDirection` _direction
        (:`Forward`
          (`self.Backward`))
        (:`Backward`
          (`self.Forward`))))))

(event `Forward`
  ;[1 1 1] Movement Mechanism & Initialize Sprite Type
  (goto _label))

(event `Backward`
  ;[1 1 1] Movement Mechanism & Initialize Sprite Type
  (goto _label :!via `Reverse`))

(fn `UserConstructionScript`)