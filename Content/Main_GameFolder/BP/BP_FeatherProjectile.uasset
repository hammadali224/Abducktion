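; Feather projectile instigated by BP_WhiteDuck that damages foxes and the final boss.
; Separate overlap components handle each target: Capsule checks for BP_Fox and Boss checks for BP_FinalBoss.
; A valid hit applies the instigating duck's AttackPower as damage and destroys the projectile.
; A timer started on BeginPlay destroys it after a few seconds if it hits neither.
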(event `self.ReceiveBeginPlay`
  (`KismetSystemLibrary.K2_SetTimer` null "DestroyProjectile" 4.0))

(event `self.Capsule.OnComponentBeginOverlap`
  (params (OverlappedComponent :type "PrimitiveComponent Object Reference") (OtherActor :type "Actor Object Reference") (OtherComp :type "PrimitiveComponent Object Reference") (OtherBodyIndex :type Integer) (bFromSweep :type Boolean) (SweepResult :type "HitResult Structure (by ref)"))
  (bind _asbp_white_duck (cast `/Game/Main_GameFolder/BP/BP_WhiteDuck` (`self.GetInstigator`)))
  (bind _asbp_fox (cast `/Game/Main_GameFolder/BP/BP_Fox` OtherActor))
  (`GameplayStatics.ApplyDamage` _asbp_fox (`/Game/Main_GameFolder/BP/BP_WhiteDuck.AttackPower` _asbp_white_duck) null null "/Script/Engine.DamageType")
  (`self.K2_DestroyActor`))

(event `self.boss.OnComponentBeginOverlap`
  (params (OverlappedComponent :type "PrimitiveComponent Object Reference") (OtherActor :type "Actor Object Reference") (OtherComp :type "PrimitiveComponent Object Reference") (OtherBodyIndex :type Integer) (bFromSweep :type Boolean) (SweepResult :type "HitResult Structure (by ref)"))
  (bind _asbp_white_duck (cast `/Game/Main_GameFolder/BP/BP_WhiteDuck` (`self.GetInstigator`)))
  (bind _asbp_final_boss (cast `/Game/Main_GameFolder/BP/BP_FinalBoss` OtherActor))
  (`GameplayStatics.ApplyDamage` _asbp_final_boss (`/Game/Main_GameFolder/BP/BP_WhiteDuck.AttackPower` _asbp_white_duck) null null "/Script/Engine.DamageType")
  (`self.K2_DestroyActor`))

(fn `DestroyProjectile`
  (`self.K2_DestroyActor`))

(fn `UserConstructionScript`)