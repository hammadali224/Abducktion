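; Final boss for a 2D flipbook game that patrols, shoots and shows the win screen, pausing the game, when killed.
; A ping-pong timeline lerps its box toward MovementLocation and back, flipping the sprite and reversing early on bottom overlap.
; A self-repeating delayed event fires projectiles from the arrow matching its facing.
; Box hits damage and launch BP_WhiteDuck, while a state-to-flipbook function shows idle, attack, hit and death.
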(event `self.ReceiveTick`
  (params (DeltaSeconds :type "Float (single-precision)")))

(event `ShootProjectile`
  ;[1 1 1] Shoot player
  (if (`self.isFacingRight`)
    (`|SpawnActorFromClass` "/Game/Main_GameFolder/BP/BP_FinalBossProjectile.BP_FinalBossProjectile_C" (`SceneComponent.K2_GetComponentToWorld` (`self.Arrow`)) "Undefined" "OverrideRootScale" null null)
    (else
      (`|SpawnActorFromClass` "/Game/Main_GameFolder/BP/BP_FinalBossProjectile.BP_FinalBossProjectile_C" (`SceneComponent.K2_GetComponentToWorld` (`self.ArrowOpp`)) "Undefined" "OverrideRootScale" null null)))
  (`self.Set Flip Book` "NewEnumerator2")
  (`KismetSystemLibrary.Delay` 1.0)
  (`self.Set Flip Book` "NewEnumerator0")
  (`self.ShootProjectile`))

(event `self.Bottom.OnComponentBeginOverlap`
  (params (OverlappedComponent :type "PrimitiveComponent Object Reference") (OtherActor :type "Actor Object Reference") (OtherComp :type "PrimitiveComponent Object Reference") (OtherBodyIndex :type Integer) (bFromSweep :type Boolean) (SweepResult :type "HitResult Structure (by ref)"))
  ;[1 1 1] Reverse Direction when bottom hits
  (if (`TimelineComponent.IsReversing` (`self.Intp`))
    (`self.Forward`)))

(event `Forward`
  ;[1 1 1] Movement Mechanism & Initialize Sprite Type
  (set `self.isFacingRight` true)
  (`self.Direction`)
  (bind (_direction _linearintp) (`Timeline|Intp` :!label _label)
    (:`Update`
      (`SceneComponent.K2_SetRelativeLocation` (`self.Box`) (`KismetMathLibrary.VLerp` (0.0 0.0 0.0) (`self.MovementLocation`) _linearintp) false false))
    (:`Finished`
      (switch `ETimelineDirection` _direction
        (:`Forward`
          (`self.Backward`))
        (:`Backward`
          (`self.Forward`))))))

(event `self.ReceiveBeginPlay`
  ;[1 1 1] Movement Mechanism & Initialize Sprite Type
  (bind _asbp_white_duck (cast `/Game/Main_GameFolder/BP/BP_WhiteDuck` (`GameplayStatics.GetPlayerCharacter` 0)))
  (set `self.Char REF` _asbp_white_duck)
  (`self.ShootProjectile`)
  (set `self.currentHealth` (`self.maxHealth`))
  (`TimelineComponent.SetPlayRate` (`self.Intp`) (/ 1.0 (`self.Duration`)))
  (goto _label :!via `PlayFromStart`))

(event `Backward`
  ;[1 1 1] Movement Mechanism & Initialize Sprite Type
  (set `self.isFacingRight` false)
  (`self.Direction`)
  (goto _label :!via `Reverse`))

(event `self.ReceiveAnyDamage`
  (params (Damage :type "Float (single-precision)") (DamageType :type "DamageType Object Reference") (InstigatedBy :type "Controller Object Reference") (DamageCauser :type "Actor Object Reference"))
  (bind _returnvalue (- (`self.currentHealth`) Damage))
  ;[1 1 1] Receive Damage
  (if (<= _returnvalue 0.0)
    (set `self.currentHealth` 0.0)
    (set `self.isDead` true)
    (`self.Set Flip Book` "NewEnumerator4")
    (`KismetSystemLibrary.Delay` 1.5)
    (`self.K2_DestroyActor`)
    (bind _returnvalue_2 (`|CreateWidget` "/Game/Main_GameFolder/BP/GameWin_Widget.GameWin_Widget_C"))
    (`UserWidget.AddToViewport` _returnvalue_2 0)
    (set `PlayerController.bShowMouseCursor` true (`GameplayStatics.GetPlayerController` 0))
    (`GameplayStatics.SetGamePaused` true)
    (else
      (set `self.currentHealth` _returnvalue)
      (`self.Set Flip Book` "NewEnumerator3")
      (`KismetSystemLibrary.Delay` 2.0)
      (`self.Set Flip Book` "NewEnumerator0"))))

(event `AnimationUpdate`
  ;[1 1 1] Receive Damage
  ;;[1 1 1] Idle or Run
  (`self.Set Flip Book` "NewEnumerator0"))

(event `Direction`
  ;[1 1 1] Facing Orientation
  (`SceneComponent.K2_SetRelativeRotation` (`self.FinalBoss`) (`KismetMathLibrary.MakeRotator` 0.0 0.0 (`KismetMathLibrary.SelectFloat` 0.0 180.0 (`self.isFacingRight`))) false false))

(event `self.Box.OnComponentHit`
  (params (HitComponent :type "PrimitiveComponent Object Reference") (OtherActor :type "Actor Object Reference") (OtherComp :type "PrimitiveComponent Object Reference") (NormalImpulse :type "Vector Structure") (Hit :type "HitResult Structure (by ref)"))
  ;[1 1 1] Cause Damage & KnockBack
  (set `self.isFacingRight` (not (`self.isFacingRight`)))
  (bind _asbp_white_duck (cast `/Game/Main_GameFolder/BP/BP_WhiteDuck` OtherActor))
  (`GameplayStatics.ApplyDamage` _asbp_white_duck (`self.BaesDamage`))
  (bind (_returnvalue_x _returnvalue_y) (`KismetMathLibrary.BreakVector` (`KismetMathLibrary.GetDirectionUnitVector` (`SceneComponent.K2_GetComponentLocation` (`self.Box`)) (`self.K2_GetActorLocation` _asbp_white_duck))))
  (bind (_returnvalue_x_2 _returnvalue_y_2 _returnvalue_z) (`KismetMathLibrary.BreakVector` (* (+ (`KismetMathLibrary.Normal` (`KismetMathLibrary.MakeVector` _returnvalue_x _returnvalue_y)) (0.0 0.0 1.0)) (`self.KnockBackSpeed`))))
  (`Character.LaunchCharacter` _asbp_white_duck (`KismetMathLibrary.MakeVector` _returnvalue_x_2 0.0 _returnvalue_z) false false))

(fn `Set Flip Book`
  (params (`Next State` :type "/Game/Main_GameFolder/WhiteDuck_Sprite/AnimStates Enum" :default "NewEnumerator0"))
  (bind _idle (`self.Idle`))
  (set `self.currentState` `Next State`)
  (`PaperFlipbookComponent.SetFlipbook` (`self.FinalBoss`) (select `/Game/Main_GameFolder/WhiteDuck_Sprite/AnimStates` (`self.currentState`) :`NewEnumerator0` _idle :`NewEnumerator1` _idle :`NewEnumerator2` (`self.Attack`) :`NewEnumerator3` (`self.Hit`) :`NewEnumerator4` (`self.Die`)))
  (return))

(fn `UserConstructionScript`)