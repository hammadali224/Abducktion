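; BP_DamagePack is a sprite-based hazard that damages and knocks back the BP_WhiteDuck character when it enters the box trigger.
; The construction script and BeginPlay both set the configurable sprite, so it also shows in the editor.
; On overlap it applies damage, then launches the duck away along the flattened direction from the pack's root plus an upward boost, scaled by KnockBackSpeed and using only X and Z.
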(event `self.ReceiveBeginPlay`
  ;[1 1 1] Initialize Sprite Type
  (`PaperSpriteComponent.SetSprite` (`self.PaperSprite`) (`self.DamagePackSprite`)))

(event `self.Box.OnComponentBeginOverlap`
  (params (OverlappedComponent :type "PrimitiveComponent Object Reference") (OtherActor :type "Actor Object Reference") (OtherComp :type "PrimitiveComponent Object Reference") (OtherBodyIndex :type Integer) (bFromSweep :type Boolean) (SweepResult :type "HitResult Structure (by ref)"))
  ;[1 1 1] Apply Damage & KnockBack
  (bind _asbp_white_duck (cast `/Game/Main_GameFolder/BP/BP_WhiteDuck` OtherActor))
  (`GameplayStatics.ApplyDamage` _asbp_white_duck (`self.DamageApply`))
  (bind (_returnvalue_x _returnvalue_y) (`KismetMathLibrary.BreakVector` (`KismetMathLibrary.GetDirectionUnitVector` (`SceneComponent.K2_GetComponentLocation` (`self.Root`)) (`self.K2_GetActorLocation` _asbp_white_duck))))
  (bind (_returnvalue_x_2 _returnvalue_y_2 _returnvalue_z) (`KismetMathLibrary.BreakVector` (* (+ (`KismetMathLibrary.Normal` (`KismetMathLibrary.MakeVector` _returnvalue_x _returnvalue_y)) (0.0 0.0 1.0)) (`self.KnockBackSpeed`))))
  (`Character.LaunchCharacter` _asbp_white_duck (`KismetMathLibrary.MakeVector` _returnvalue_x_2 0.0 _returnvalue_z) false false))

(fn `UserConstructionScript`
  ;[1 1 1] Allow Sprite Visual before Play
  (`PaperSpriteComponent.SetSprite` (`self.PaperSprite`) (`self.DamagePackSprite`)))