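; BP_Fox is a 2D flipbook enemy that walks along the X axis and reverses direction whenever its capsule hits something.
; Tick drives movement and sprite facing, and picks idle or run from velocity through SetFlipBook.
; Hitting BP_WhiteDuck deals damage and launches it up and away.
; AnyDamage reduces health, and at zero sets the die flipbook and destroys the fox after a delay, though Tick keeps updating animation meanwhile.
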(event `self.ReceiveBeginPlay`
  (set `self.CurrentHealth` (`self.MaxHealth`)))

(event `self.ReceiveTick`
  (params (DeltaSeconds :type "Float (single-precision)"))
  ;[1 1 1] Animation Update
  (`self.Direction`)
  (`self.AnimationUpdate`))

(event `self.ReceiveAnyDamage`
  (params (Damage :type "Float (single-precision)") (DamageType :type "DamageType Object Reference") (InstigatedBy :type "Controller Object Reference") (DamageCauser :type "Actor Object Reference"))
  (bind _returnvalue (- (`self.CurrentHealth`) Damage))
  ;[1 1 1] Receive Damage
  (if (<= _returnvalue 0.0)
    (set `self.CurrentHealth` 0.0)
    (set `self.isDead` true)
    (`self.SetFlipBook` "NewEnumerator4")
    (`KismetSystemLibrary.Delay` 1.5)
    (`self.K2_DestroyActor`)
    (else
      (set `self.CurrentHealth` _returnvalue))))

(event `AnimationUpdate`
  ;[1 1 1] Idle or Run
  (`self.SetFlipBook` (select `bool` (> (`KismetMathLibrary.VSize` (`self.GetVelocity`)) 0.0) :`false` "NewEnumerator0" :`true` "NewEnumerator1" :!type "/Game/Main_GameFolder/WhiteDuck_Sprite/AnimStates Enum")))

(event `Direction`
  ;[1 1 1] Facing Orientation
  (`SceneComponent.K2_SetRelativeRotation` (`self.Sprite`) (`KismetMathLibrary.MakeRotator` 0.0 0.0 (`KismetMathLibrary.SelectFloat` 0.0 180.0 (`self.isMovingRight`))) false false)
  (`self.AddMovementInput` (`KismetMathLibrary.SelectVector` (1.0 0.0 0.0) (-1.0 0.0 0.0) (`self.isMovingRight`))))

(event `self.CapsuleComponent.OnComponentHit`
  (params (HitComponent :type "PrimitiveComponent Object Reference") (OtherActor :type "Actor Object Reference") (OtherComp :type "PrimitiveComponent Object Reference") (NormalImpulse :type "Vector Structure") (Hit :type "HitResult Structure (by ref)"))
  ;[1 1 1] Cause Damage & KnockBack
  (set `self.isMovingRight` (not (`self.isMovingRight`)))
  (bind _asbp_white_duck (cast `/Game/Main_GameFolder/BP/BP_WhiteDuck` OtherActor))
  (`GameplayStatics.ApplyDamage` _asbp_white_duck (`self.BaseDamage`))
  (bind (_returnvalue_x _returnvalue_y) (`KismetMathLibrary.BreakVector` (`KismetMathLibrary.GetDirectionUnitVector` (`SceneComponent.K2_GetComponentLocation` (`self.CapsuleComponent`)) (`self.K2_GetActorLocation` _asbp_white_duck))))
  (bind (_returnvalue_x_2 _returnvalue_y_2 _returnvalue_z) (`KismetMathLibrary.BreakVector` (* (+ (`KismetMathLibrary.Normal` (`KismetMathLibrary.MakeVector` _returnvalue_x _returnvalue_y)) (0.0 0.0 1.0)) (`self.KnockBackSpeed`))))
  (`self.LaunchCharacter` _asbp_white_duck (`KismetMathLibrary.MakeVector` _returnvalue_x_2 0.0 _returnvalue_z) false false))

(fn `ChangeHealth`
  (params (Amount :type "Float (double-precision)"))
  (bind _returnvalue (+ Amount (`self.CurrentHealth`)))
  (if (<= _returnvalue (`self.MaxHealth`))
    (set `self.CurrentHealth` _returnvalue)
    (else
      (set `self.CurrentHealth` (`self.MaxHealth`)))))

(fn `SetFlipBook`
  (params (NextState :type "/Game/Main_GameFolder/WhiteDuck_Sprite/AnimStates Enum" :default "NewEnumerator0"))
  (set `self.currentState` NextState)
  (`PaperFlipbookComponent.SetFlipbook` (`self.Sprite`) (select `/Game/Main_GameFolder/WhiteDuck_Sprite/AnimStates` (`self.currentState`) :`NewEnumerator0` (`self.FB_Idel`) :`NewEnumerator1` (`self.FB_Run`) :`NewEnumerator2` (`self.FB_Jump`) :`NewEnumerator3` (`self.FB_Fly`) :`NewEnumerator4` (`self.FB_Die`)))
  (return))

(fn `UserConstructionScript`)