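; BP_Door is a Paper2D sprite door that serves as a level exit for BP_WhiteDuck.
; The construction script and BeginPlay both set the DoorSprite variable as the sprite.
; When the duck overlaps CollisionBox, the sprite changes and, after a short delay, FirstHUD's LevelEnd runs and player move input is ignored.
; After a further delay it opens the level named by NewLevel.
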(event `self.ReceiveBeginPlay`
  (`PaperSpriteComponent.SetSprite` (`self.PaperSprite`) (`self.DoorSprite`)))

(event `self.CollisionBox.OnComponentBeginOverlap`
  (params (OverlappedComponent :type "PrimitiveComponent Object Reference") (OtherActor :type "Actor Object Reference") (OtherComp :type "PrimitiveComponent Object Reference") (OtherBodyIndex :type Integer) (bFromSweep :type Boolean) (SweepResult :type "HitResult Structure (by ref)"))
  (bind _returnvalue (`GameplayStatics.GetPlayerController` 0))
  (cast `/Game/Main_GameFolder/BP/BP_WhiteDuck` OtherActor)
  (`PaperSpriteComponent.SetSprite` (`self.PaperSprite`) "/Game/Main_GameFolder/Door_Sprite/Open/05_Sprite_0.05_Sprite_0")
  (`KismetSystemLibrary.Delay` 0.25)
  (bind _asfirst_hud (cast `/Game/Main_GameFolder/BP/GameMode/FirstHUD` (`PlayerController.GetHUD` _returnvalue)))
  (`|ExecutionSequence`
    (:`then_0`
      (`/Game/Main_GameFolder/BP/GameMode/FirstHUD.LevelEnd` _asfirst_hud)
      (`Controller.SetIgnoreMoveInput` _returnvalue true))
    (:`then_1`
      (`KismetSystemLibrary.Delay` 1.0)
      (`GameplayStatics.OpenLevel` (`self.NewLevel`)))))

(fn `UserConstructionScript`
  (`PaperSpriteComponent.SetSprite` (`self.PaperSprite`) (`self.DoorSprite`)))