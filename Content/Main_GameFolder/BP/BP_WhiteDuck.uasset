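; BP_WhiteDuck is the player-controlled 2D duck character for a side-scrolling game, with running, jumping and feather shooting.
; Tick sets controller yaw from X velocity or last input direction, while a state enum selects flipbooks through SetFlipBook.
; Damage reduces health until RestartGame plays the death flipbook, disables input and shows a paused game-over screen.
; It also toggles the pause menu and exposes health and attack-power modifier functions.
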(event `self.ReceiveBeginPlay`
  ;[1 1 1] Initialize Health
  (set `self.CurrentHealth` (`self.MaxHealth`)))

(event `self.ReceiveTick`
  (params (DeltaSeconds :type "Float (single-precision)"))
  ;[1 1 1] Animation Update
  (`self.Direction`)
  (`self.AnimationUpdate`))

(event `InputAxis|MoveRight`
  (params (AxisValue :type "Float (single-precision)"))
  ;[1 1 1] Move Mechanic
  (`/Engine/EditorBlueprintResources/StandardMacros.CompareFloat` AxisValue
    (:`>`
      (set `self.isMovingRight` true))
    (:`<`
      (set `self.isMovingRight` false)))
  (`self.AddMovementInput` (1.0 0.0 0.0) AxisValue))

(event `Direction`
  (bind _returnvalue_x (`KismetMathLibrary.BreakVector` (`self.GetVelocity`)))
  (bind _returnvalue (`self.GetController`))
  ;[1 1 1] Facing Orientation
  (`/Engine/EditorBlueprintResources/StandardMacros.CompareFloat` _returnvalue_x
    (:`>`
      (`Controller.SetControlRotation` _returnvalue (`KismetMathLibrary.MakeRotator` 0.0) :!label _label))
    (:`==`
      (if (`self.isMovingRight`)
        (goto _label)
        (else
          (`Controller.SetControlRotation` _returnvalue (`KismetMathLibrary.MakeRotator` 0.0 0.0 180.0) :!label _label_2))))
    (:`<`
      (goto _label_2))))

(event `InputAction|Jump`
  (params (Key :type "Key Structure"))
  ;[1 1 1] Jump Mechanic
  (:`Pressed`
    (`self.Jump`)
    (if (`self.CanJump`)
      (`self.SetFlipBook` "NewEnumerator2")
      (`KismetSystemLibrary.Delay` 1.0)
      (if (`NavMovementComponent.IsFalling` (`self.CharacterMovement`))
        (`self.SetFlipBook` "NewEnumerator3"))))
  (:`Released`
    (`self.StopJumping`)))

(event `AnimationUpdate`
  ;[1 1 1] Idle or Run
  (if (`NavMovementComponent.IsFalling` (`self.CharacterMovement`))
    _
    (elif (not (`self.isDead`))
      (`self.SetFlipBook` (select `bool` (> (`KismetMathLibrary.VSize` (`self.GetVelocity`)) 0.0) :`false` "NewEnumerator0" :`true` "NewEnumerator1" :!type "/Game/Main_GameFolder/WhiteDuck_Sprite/AnimStates Enum")))))

(event `Key|Escape` :paused true
  (params (Key :type "Key Structure"))
  ;[1 1 1] Pause Game
  (:`Pressed`
    (`/Engine/EditorBlueprintResources/StandardMacros.FlipFlop`
      (:`A`
        (`GameplayStatics.SetGamePaused` true)
        (bind _returnvalue (`|CreateWidget` "/Game/Main_GameFolder/BP/GamePause_Widget.GamePause_Widget_C"))
        (`UserWidget.AddToViewport` _returnvalue 0)
        (set `PlayerController.bShowMouseCursor` true (`GameplayStatics.GetPlayerController` 0)))
      (:`B`
        (`Widget.RemoveFromParent` _returnvalue)
        (`GameplayStatics.SetGamePaused` false)
        (set `PlayerController.bShowMouseCursor` false (`GameplayStatics.GetPlayerController` 0))))))

(event `Restart Game`
  ;[1 1 1] Die & Restart
  (set `self.isDead` true)
  (`self.DisableInput` (`GameplayStatics.GetPlayerController` 0))
  (`self.SetFlipBook` "NewEnumerator4")
  (`KismetSystemLibrary.Delay` 0.5)
  (bind _returnvalue (`|CreateWidget` "/Game/Main_GameFolder/BP/GameOver_Widget.GameOver_Widget_C"))
  (`UserWidget.AddToViewport` _returnvalue 0)
  (set `PlayerController.bShowMouseCursor` true (`GameplayStatics.GetPlayerController` 0))
  (`GameplayStatics.SetGamePaused` true))

(event `self.ReceiveAnyDamage`
  (params (Damage :type "Float (single-precision)") (DamageType :type "DamageType Object Reference") (InstigatedBy :type "Controller Object Reference") (DamageCauser :type "Actor Object Reference"))
  (bind _returnvalue (- (`self.CurrentHealth`) Damage))
  ;[1 1 1] Receive Damage
  (if (<= _returnvalue 0.0)
    (set `self.CurrentHealth` 0.0)
    (`self.Restart Game`)
    (else
      (set `self.CurrentHealth` _returnvalue))))

(event `Key|S`
  (params (Key :type "Key Structure"))
  ;[1 1 1] Shoot Projectile
  (:`Pressed`
    (`|SpawnActorFromClass` "/Game/Main_GameFolder/BP/BP_FeatherProjectile.BP_FeatherProjectile_C" (`SceneComponent.K2_GetComponentToWorld` (`self.ArrowShot`)) "Undefined" "OverrideRootScale" null null)))

(fn `ChangeHealth`
  (params (Amount :type "Float (double-precision)"))
  (bind _returnvalue (+ Amount (`self.CurrentHealth`)))
  (if (<= _returnvalue (`self.MaxHealth`))
    (set `self.CurrentHealth` _returnvalue)
    (else
      (set `self.CurrentHealth` (`self.MaxHealth`)))))

(fn `DecreaseAttackPower`
  (params (AttackPowerChange :type "Float (double-precision)"))
  (set `self.AttackPower` (- AttackPowerChange (`self.AttackPower`))))

(fn `IncreaseAttackPower`
  (params (AttackPowerAmount :type "Float (double-precision)"))
  (set `self.AttackPower` (+ AttackPowerAmount (`self.AttackPower`))))

(fn `SetFlipBook`
  (params (NextState :type "/Game/Main_GameFolder/WhiteDuck_Sprite/AnimStates Enum" :default "NewEnumerator0"))
  (set `self.currentState` NextState)
  (`PaperFlipbookComponent.SetFlipbook` (`self.Sprite`) (select `/Game/Main_GameFolder/WhiteDuck_Sprite/AnimStates` (`self.currentState`) :`NewEnumerator0` (`self.FB_Idel`) :`NewEnumerator1` (`self.FB_Run`) :`NewEnumerator2` (`self.FB_Jump`) :`NewEnumerator3` (`self.FB_Fly`) :`NewEnumerator4` (`self.FB_Die`)))
  (return))

(fn `UserConstructionScript`)