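; BP_HealthPack is a health pickup shown as a spinning, bobbing Paper2D sprite.
; When BP_WhiteDuck begins overlapping its Box, it passes HealthRestore to the duck's ChangeHealth and destroys itself.
; The SpinAndBob timeline drives the sprite's relative height and yaw from BeginPlay, restarting through PlayAnimation whenever it finishes.
; The construction script applies HealthPackSprite so the pack is visible before play.
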(event `self.Box.OnComponentBeginOverlap`
  (params (OverlappedComponent :type "PrimitiveComponent Object Reference") (OtherActor :type "Actor Object Reference") (OtherComp :type "PrimitiveComponent Object Reference") (OtherBodyIndex :type Integer) (bFromSweep :type Boolean) (SweepResult :type "HitResult Structure (by ref)"))
  ;[1 1 1] Add Health
  (bind _asbp_white_duck (cast `/Game/Main_GameFolder/BP/BP_WhiteDuck` OtherActor))
  (`/Game/Main_GameFolder/BP/BP_WhiteDuck.ChangeHealth` _asbp_white_duck (`self.HealthRestore`))
  (`self.K2_DestroyActor`))

(event `PlayAnimation`
  ;[1 1 1] Initialize Sprite & Motion Animation
  (bind (_direction _position _rotation) (`Timeline|Spin and Bob` :!via `PlayFromStart` :!label _label)
    (:`Update`
      (`SceneComponent.K2_SetRelativeLocationAndRotation` (`self.PaperSprite`) (`KismetMathLibrary.MakeVector` 0.0 0.0 _position) (`KismetMathLibrary.MakeRotator` 0.0 0.0 _rotation) false false))
    (:`Finished`
      (`self.PlayAnimation`))))

(event `self.ReceiveBeginPlay`
  ;[1 1 1] Initialize Sprite & Motion Animation
  (`PaperSpriteComponent.SetSprite` (`self.PaperSprite`) (`self.HealthPackSprite`))
  (goto _label :!via `PlayFromStart`))

(fn `UserConstructionScript`
  ;[1 1 1] Allow visual of sprite before play
  (`PaperSpriteComponent.SetSprite` (`self.PaperSprite`) (`self.HealthPackSprite`)))